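; Security agent character with a melee attack against BP_TopDownCharacter and a colored alert circle.
; MeleeAttack plays a montage and punch sound, then uses its Notify Begin to sphere-overlap at the Sphere component and damage any player character found.
; The construction script and Alert event each create a dynamic material on AlertCircle and apply the ColorAlert tint.
; A debug sphere draw for the attack radius is left unconnected.
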(event `/Game/SecurityAgent/AI/INT_Combat.MeleeAttack`
  ;[1 1 1] Animation d'attaque
  (`|PlayMontage` (`self.Mesh`) "/Game/SecurityAgent/Animations/MontageAttack.MontageAttack"
    (:`then`
      ;;[1 1 1] Points de vie
      (`GameplayStatics.PlaySound2D` "/Game/Audio/Punch-sound-effect.Punch-sound-effect" 0.1 1.0 0.0 null null))
    (:`OnNotifyBegin`
      (bind _outactors (`KismetSystemLibrary.SphereOverlapActors` (`SceneComponent.K2_GetComponentLocation` (`self.Sphere`)) (`self.Attack Sphere Radius`) (`|MakeArray` "ObjectTypeQuery3" :!type "EObjectTypeQuery Enum") "/Game/TopDown/Blueprints/BP_TopDownCharacter.BP_TopDownCharacter_C" (`|MakeArray` self :!type "Actor Object Reference")))
      (for _array_element _outactors
        (`GameplayStatics.ApplyDamage` _array_element (`self.Attack Base Damage`) (`self.GetController`) self "/Script/Engine.DamageType")))))

(event `Event Alert`
  (bind _returnvalue (`PrimitiveComponent.CreateDynamicMaterialInstance` (`self.AlertCircle`) 0 "/Game/SecurityAgent/Material/Alert_Circle.Alert_Circle" "None"))
  (`MaterialInstanceDynamic.SetVectorParameterValue` _returnvalue "ColorAlert" (`self.ColorAlert`)))

(fn `UserConstructionScript`
  (bind _returnvalue (`PrimitiveComponent.CreateDynamicMaterialInstance` (`self.AlertCircle`) 0 "/Game/SecurityAgent/Material/Alert_Circle.Alert_Circle" "None"))
  (`MaterialInstanceDynamic.SetVectorParameterValue` _returnvalue "ColorAlert" (`self.ColorAlert`)))