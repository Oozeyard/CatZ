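; BP_Monster1 is a monster character with a melee attack, noisy footsteps and a randomized modular outfit.
; MeleeAttack plays a montage whose notify runs a sphere overlap, damaging BP_Cat pawns with a punch sound.
; Footsteps scale volume and AI noise reports by velocity relative to the walk speed cached at BeginPlay.
; The Construction Script links outfit meshes to the body through Leader Pose and randomly toggles each one's visibility.
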(event `/Game/SecurityAgent/AI/INT_Combat.MeleeAttack`
  ;[1 1 1] Animation d'attaque
  (`|PlayMontage` (`self.Mesh`) "/Game/SecurityAgent/Animations/MontageAttackMonster.MontageAttackMonster"
    (:`OnNotifyBegin`
      ;;[1 1 1] Points de vie
      (bind _outactors (`KismetSystemLibrary.SphereOverlapActors` (`SceneComponent.K2_GetComponentLocation` (`self.Sphere`)) (`self.Attack Sphere Radius`) (`|MakeArray` "ObjectTypeQuery3" :!type "EObjectTypeQuery Enum") "/Game/Cats/BP_Cat.BP_Cat_C" (`|MakeArray` self :!type "Actor Object Reference")))
      (for _array_element _outactors
        (`GameplayStatics.ApplyDamage` _array_element (`self.Attack Base Damage`) (`self.GetController`) self "/Script/Engine.DamageType")
        (`GameplayStatics.PlaySound2D` "/Game/Audio/Punch-sound-effect.Punch-sound-effect" 0.1 1.0 0.0 null null)))))

(event `self.ReceiveBeginPlay`
  (set `self.SprintSpeed` (`CharacterMovementComponent.MaxWalkSpeed` (`self.CharacterMovement`))))

(event `Footstep`
  (bind _returnvalue (`self.K2_GetActorLocation`))
  (bind _stepfootvolume (`self.StepFootVolume`))
  (set `self.StepFootVolume` (/ (`KismetMathLibrary.VSize` (`self.GetVelocity`)) (`self.SprintSpeed`)))
  (`GameplayStatics.PlaySoundAtLocation` "/Game/Audio/MS_Footstep.MS_Footstep" _returnvalue (struct) (/ (`self.StepFootVolume`) 5.0) 1.0 0.0 null null null null)
  (`AISense_Hearing.ReportNoiseEvent` _returnvalue _stepfootvolume self (* _stepfootvolume 500.0)))

(fn `UserConstructionScript`
  (`SkinnedMeshComponent.SetLeaderPoseComponent` (`self.Armor`) (`self.Mesh`) true false)
  (`SkinnedMeshComponent.SetLeaderPoseComponent` (`self.Belt`) (`self.Mesh`) true false)
  (`SkinnedMeshComponent.SetLeaderPoseComponent` (`self.Boots`) (`self.Mesh`) true false)
  (`SkinnedMeshComponent.SetLeaderPoseComponent` (`self.Mask`) (`self.Mesh`) true false)
  (`SkinnedMeshComponent.SetLeaderPoseComponent` (`self.Neck_Rope`) (`self.Mesh`) true false)
  (`SkinnedMeshComponent.SetLeaderPoseComponent` (`self.Rag`) (`self.Mesh`) true false)
  (`SkinnedMeshComponent.SetLeaderPoseComponent` (`self.Arrows`) (`self.Mesh`) true false)
  (`SkinnedMeshComponent.SetLeaderPoseComponent` (`self.Pants`) (`self.Mesh`) true false)
  (`SkinnedMeshComponent.SetLeaderPoseComponent` (`self.Hair`) (`self.Mesh`) true false)
  (`|ExecutionSequence`
    (:`then_0`
      (`SceneComponent.SetVisibility` (`self.Rag`) (`KismetMathLibrary.RandomBool`) false))
    (:`then_1`
      (`SceneComponent.SetVisibility` (`self.Pants`) (`KismetMathLibrary.RandomBool`) false))
    (:`then_2`
      (`SceneComponent.SetVisibility` (`self.Neck_Rope`) (`KismetMathLibrary.RandomBool`) false))
    (:`then_3`
      (`SceneComponent.SetVisibility` (`self.Mask`) (`KismetMathLibrary.RandomBool`) false))
    (:`then_4`
      (`SceneComponent.SetVisibility` (`self.Hair`) (`KismetMathLibrary.RandomBool`) false))
    (:`then_5`
      (`SceneComponent.SetVisibility` (`self.Boots`) (`KismetMathLibrary.RandomBool`) false))
    (:`then_6`
      (`SceneComponent.SetVisibility` (`self.Belt`) (`KismetMathLibrary.RandomBool`) false))
    (:`then_7`
      (`SceneComponent.SetVisibility` (`self.Arrows`) (`KismetMathLibrary.RandomBool`) false))
    (:`then_8`
      (`SceneComponent.SetVisibility` (`self.Armor`) (`KismetMathLibrary.RandomBool`) false))))