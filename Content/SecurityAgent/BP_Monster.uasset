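; BP_Monster is an enemy character that attacks BP_Cat with a melee move and makes audible footsteps.
; MeleeAttack plays a montage whose notify triggers a sphere overlap at the Sphere component, applying damage and a punch sound for each cat hit.
; Footstep plays a sound at the actor and reports an AI noise event, with both volume and range scaled by StepFootVolume.
; A debug sphere draw for the attack area is left unconnected.
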(event `/Game/SecurityAgent/AI/INT_Combat.MeleeAttack`
  ;[1 1 1] Animation d'attaque
  (`|PlayMontage` (`self.Mesh`) "/Game/SecurityAgent/Animations/MontageAttackMonster.MontageAttackMonster"
    (:`OnNotifyBegin`
      ;;[1 1 1] Points de vie
      (bind _outactors (`KismetSystemLibrary.SphereOverlapActors` (`SceneComponent.K2_GetComponentLocation` (`self.Sphere`)) (`self.Attack Sphere Radius`) (`|MakeArray` "ObjectTypeQuery3" :!type "EObjectTypeQuery Enum") "/Game/Cats/BP_Cat.BP_Cat_C" (`|MakeArray` self :!type "Actor Object Reference")))
      (for _array_element _outactors
        (`GameplayStatics.ApplyDamage` _array_element (`self.Attack Base Damage`) (`self.GetController`) self "/Script/Engine.DamageType")
        (`GameplayStatics.PlaySound2D` "/Game/Audio/Punch-sound-effect.Punch-sound-effect" 0.1 1.0 0.0 null null)))))

(event `Footstep`
  (bind _returnvalue (`self.K2_GetActorLocation`))
  (bind _step_foot_volume (`self.Step Foot Volume`))
  (set `self.Step Foot Volume` (`self.Step Foot Volume`))
  (`GameplayStatics.PlaySoundAtLocation` "/Game/Audio/footstep_Cue.footstep_Cue" _returnvalue (struct) (/ (`self.Step Foot Volume`) 5.0) 1.0 0.0 null null null null)
  (`AISense_Hearing.ReportNoiseEvent` _returnvalue _step_foot_volume self (* _step_foot_volume 2000.0)))

(fn `UserConstructionScript`
  (`parent.UserConstructionScript`))