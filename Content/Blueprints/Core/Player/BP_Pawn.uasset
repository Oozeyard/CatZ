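; Player camera pawn that pans, rotates and zooms, and can switch the view to AIC_Security AI controllers' view targets.
; Inputs update desired location, yaw and clamped spring arm length, which Tick smoothly interpolates toward.
; PossesAI toggles a blended view between the selected AI and this pawn, without actual possession.
; Index up/down inputs cycle through those AIs with wraparound and blend to the selected one.
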(event `self.ReceiveBeginPlay`
  ;[1 1 1] Sauvegarde la position, la rotation de base du player et le zoom
  (set `self.Location_Desired` (`self.K2_GetActorLocation`))
  (set `self.Zoom_Desired` (`SpringArmComponent.TargetArmLength` (`self.SpringArm`)))
  (set `self.Rotation_Desired` (`self.K2_GetActorRotation`)))

(event `self.ReceiveTick`
  (params (DeltaSeconds :type "Float (single-precision)"))
  (bind _springarm (`self.SpringArm`))
  ;[1 1 1] Event appelé à chaque frame
  ;[1 1 1] Adapte la longueur du bras de la caméra selon la valeur de zoom récupéree de manière smooth
  (set `SpringArmComponent.TargetArmLength` (`KismetMathLibrary.FInterpTo` (`SpringArmComponent.TargetArmLength` _springarm) (`self.Zoom_Desired`) DeltaSeconds (`self.ZoomInterp`)) _springarm)
  ;[1 1 1] Adapte la position du player selon la valeur de position récupérée des inputs
  (`self.K2_SetActorLocation` (`KismetMathLibrary.VInterpTo` (`self.K2_GetActorLocation`) (`self.Location_Desired`) DeltaSeconds (`self.LocationInterp`)))
  ;[1 1 1] Adapte la rotation du player selon la valeur de la rotation récupérée des inputs
  (`self.K2_SetActorRotation` (`KismetMathLibrary.RInterpTo` (`self.K2_GetActorRotation`) (`self.Rotation_Desired`) DeltaSeconds (`self.RotationInterp`))))

(event `InputAxis|InputAxis_Zoom`
  (params (AxisValue :type "Float (single-precision)"))
  ;[1 1 1] Récupère la valeur de zoom de la molette de la souris
  (set `self.Zoom_Desired` (`KismetMathLibrary.FClamp` (+ (* AxisValue (`self.ZoomSpeed`)) (`self.Zoom_Desired`)) (`self.ZoomMin`) (`self.ZoomMax`))))

(event `InputAxis|InputAxis_Forward`
  (params (AxisValue :type "Float (single-precision)"))
  ;[1 1 1] Modifie la valeur de l'axe X de la Location_Desired
  (set `self.Location_Desired` (+ (`self.Location_Desired`) (* (`self.GetActorForwardVector`) (* AxisValue (`self.LocationSpeed`))))))

(event `InputAction|PossesAI`
  (params (Key :type "Key Structure"))
  (:`Pressed`
    (`/Engine/EditorBlueprintResources/StandardMacros.FlipFlop`
      (:`A`
        (`self.GoToAIViewpoint`))
      (:`B`
        (`PlayerController.SetViewTargetWithBlend` (`GameplayStatics.GetPlayerController` 0) self 1.0 "VTBlend_Cubic" 0.0 false)))))

(event `InputAxis|InputAxis_Right`
  (params (AxisValue :type "Float (single-precision)"))
  ;[1 1 1] Modifie la valeur de l'axe Y de la Location_Desired
  (set `self.Location_Desired` (+ (`self.Location_Desired`) (* (`self.GetActorRightVector`) (* AxisValue (`self.LocationSpeed`))))))

(event `InputAction|AIPossesIdxUp`
  (params (Key :type "Key Structure"))
  (:`Pressed`
    (bind _outactors (`GameplayStatics.GetAllActorsOfClass` "/Game/SecurityAgent/AI/AIC_Security.AIC_Security_C"))
    (bind _result (`/Engine/EditorBlueprintResources/StandardMacros.IncrementInt` (`self.AIToPossesId`))
      (:`  `
        (if (> _result (- (`KismetArrayLibrary.Array_Length` _outactors) 1))
          (set `self.AIToPossesId` 0))
        (`self.GoToAIViewpoint` :!label _label)))))

(event `InputAction|AIPossesIdxDown`
  (params (Key :type "Key Structure"))
  (:`Pressed`
    (bind _result (`/Engine/EditorBlueprintResources/StandardMacros.DecrementInt` (`self.AIToPossesId`))
      (:`  `
        (if (< _result 0)
          (set `self.AIToPossesId` (- (`KismetArrayLibrary.Array_Length` (stale `InputAction|AIPossesIdxUp` _outactors)) 1))
          (goto _label)
          (else
            (goto _label)))))))

(event `InputAction|InputAction_RotationRight`
  (params (Key :type "Key Structure"))
  ;[1 1 1] Modifie la valeur de l'axe Z de la Rotation_Desired
  (:`Pressed`
    (set `self.Rotation_Desired` (`KismetMathLibrary.ComposeRotators` (`self.Rotation_Desired`) (`KismetMathLibrary.MakeRotator` 0.0 0.0 (* -1 (`self.RotationSpeed`)))))))

(event `InputAction|InputAction_RotationLeft`
  (params (Key :type "Key Structure"))
  ;[1 1 1] Modifie la valeur de l'axe Z de la Rotation_Desired
  (:`Pressed`
    (set `self.Rotation_Desired` (`KismetMathLibrary.ComposeRotators` (`self.Rotation_Desired`) (`KismetMathLibrary.MakeRotator` 0.0 0.0 (`self.RotationSpeed`))))))

(fn `GoToAIViewpoint`
  (bind _aitopossesid (`self.AIToPossesId`))
  (bind _outactors (`GameplayStatics.GetAllActorsOfClass` "/Game/SecurityAgent/AI/AIC_Security.AIC_Security_C"))
  (if (`KismetArrayLibrary.Array_IsValidIndex` _outactors _aitopossesid)
    (`PlayerController.SetViewTargetWithBlend` (`GameplayStatics.GetPlayerController` 0) (`Controller.GetViewTarget` (`|GetArrayItem` _outactors _aitopossesid)) 2.0 "VTBlend_Cubic" 0.0 false)))

(fn `UserConstructionScript`)