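; BP_Score runs the match countdown and decides the outcome between the Zombie and Cat sides.
; A one-second Delay on Tick throttles the countdown, stepping Seconds down and rolling over Minutes.
; At zero it pauses the game, compares ZScore with CScore, and adds the zombie victory, cat victory or draw widget to the viewport.
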(event `self.ReceiveTick`
  (params (DeltaSeconds :type "Float (single-precision)"))
  (`KismetSystemLibrary.Delay` 1.0)
  (if (== (`self.Seconds`) 0)
    (if (== (`self.Minutes`) 0)
      (`GameplayStatics.SetGamePaused` true)
      (if (== (`self.ZScore`) (`self.CScore`))
        (bind _returnvalue (`|CreateWidget` "/Game/ScoreUI/Draw_WIDGET.Draw_WIDGET_C"))
        (`UserWidget.AddToViewport` _returnvalue 0)
        (elif (> (`self.ZScore`) (`self.CScore`))
          (bind _returnvalue_2 (`|CreateWidget` "/Game/ScoreUI/ZombieVictory_WIDGET.ZombieVictory_WIDGET_C"))
          (`UserWidget.AddToViewport` _returnvalue_2 0)
          (else
            (bind _returnvalue_3 (`|CreateWidget` "/Game/ScoreUI/CatVictory_WIDGET.CatVictory_WIDGET_C"))
            (`UserWidget.AddToViewport` _returnvalue_3 0))))
      (else
        (set `self.Minutes` (- (`self.Minutes`) 1))
        (set `self.Seconds` 59)))
    (else
      (set `self.Seconds` (- (`self.Seconds`) 1)))))

(fn `UserConstructionScript`)