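; Milk pickup that a cat collects on capsule overlap, calling GetMilk on the cat and adding to the score in BP_Score.
; On pickup it spawns a replacement at a random navigable location around the farthest MilkRespawnArea target point, then destroys itself.
; The farthest point is found by repeatedly removing the nearest one from the list.
; While targeted, it draws a debug box around itself each tick.
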(event `self.ReceiveTick`
  (params (DeltaSeconds :type "Float (single-precision)"))
  (if (`self.isTargeted`)
    (`KismetSystemLibrary.DrawDebugBox` (`self.K2_GetActorLocation`) (50.0 50.0 50.0) (struct :`G` 1.0 :`B` 0.263449 :`A` 1.0) (struct) 0.0 5.0)))

(event `self.Capsule.OnComponentBeginOverlap`
  (params (OverlappedComponent :type "PrimitiveComponent Object Reference") (OtherActor :type "Actor Object Reference") (OtherComp :type "PrimitiveComponent Object Reference") (OtherBodyIndex :type Integer) (bFromSweep :type Boolean) (SweepResult :type "HitResult Structure (by ref)"))
  (bind _asbp_cat (cast `/Game/Cats/BP_Cat` OtherActor))
  (`/Game/Cats/BP_Cat.GetMilk` _asbp_cat)
  (bind _returnvalue (`GameplayStatics.GetActorOfClass` "/Game/UI/BP_Score.BP_Score_C"))
  (`/Game/UI/BP_Score.Update Cat Score` _returnvalue (`self.scoreIncrease`))
  (`self.respawn` (`self.respawnRadius`))
  (`self.K2_DestroyActor`))

(fn `getFurthestRespawnPoint`
  (returns (Output :type "TargetPoint Object Reference"))
  (locals (RespawnPoints :type "Array of TargetPoint Object Reference"))
  (bind _outactors (`GameplayStatics.GetAllActorsOfClassWithTag` "/Script/Engine.TargetPoint" "MilkRespawnArea"))
  (set `local.RespawnPoints` _outactors)
  (for _ (range (+ (- (`KismetArrayLibrary.Array_Length` _outactors) 2) 1))
    (bind _astarget_point (cast `TargetPoint` (`.ReturnValue` (`GameplayStatics.FindNearestActor` (`self.K2_GetActorLocation`) (`local.RespawnPoints`)))))
    (`KismetArrayLibrary.Array_RemoveItem` (`local.RespawnPoints`) _astarget_point))
  (if (`KismetArrayLibrary.Array_IsValidIndex` (`local.RespawnPoints`))
    (return (`|GetArrayItem` (`local.RespawnPoints`)))
    (else
      (`KismetSystemLibrary.PrintString` "erreur array"))))

(fn `respawn`
  (params (Radius :type "Float (single-precision)"))
  (bind _output (`self.getFurthestRespawnPoint`))
  (bind _randomlocation (`NavigationSystemV1.K2_GetRandomLocationInNavigableRadius` (`self.K2_GetActorLocation` _output) (`local.Radius`) null null))
  (`|SpawnActorFromClass` "BP_Milk_C" (`KismetMathLibrary.MakeTransform` (`KismetMathLibrary.MakeVector` (.x _randomlocation) (.y _randomlocation) 140.0)) "AdjustIfPossibleButAlwaysSpawn" "MultiplyWithRoot" null null))

(fn `UserConstructionScript`)