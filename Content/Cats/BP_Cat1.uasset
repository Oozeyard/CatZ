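; BP_Cat1 is a cat actor that dies on any damage and is replaced by a new cat, crediting the zombies' score.
; Respawn destroys it, releases its targeted milk and spawns a replacement at a random navigable point around a random TargetPoint tagged CatRespawnArea.
; The damage event then reports zombie points, survival time and the spawn to BP_Score.
; Survival time counts seconds through a one-second Delay on Tick.
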(event `self.ReceiveAnyDamage`
  (params (Damage :type "Float (single-precision)") (DamageType :type "DamageType Object Reference") (InstigatedBy :type "Controller Object Reference") (DamageCauser :type "Actor Object Reference"))
  ;[1 1 1] Respawn
  (`self.respawn`)
  ;[1 1 1] On augmente le score des zombis si un chat meurt
  (bind _returnvalue (`GameplayStatics.GetActorOfClass` "/Game/UI/BP_Score.BP_Score_C"))
  (`/Game/UI/BP_Score.Update Zombies Score` _returnvalue (`self.Zombies Score Increase_0`))
  (`/Game/UI/BP_Score.AddSurvivalTime` _returnvalue (`self.SurvialTime_0`))
  (`/Game/UI/BP_Score.UpdateCatSpawned` _returnvalue))

(event `GetMilk`)

(event `self.ReceiveTick`
  (params (DeltaSeconds :type "Float (single-precision)"))
  (`KismetSystemLibrary.Delay` 1.0)
  (set `self.SurvialTime_0` (+ (`self.SurvialTime_0`) 1)))

(event `self.ReceiveBeginPlay`)

(fn `respawn`
  (locals (Radius :type "Float (single-precision)" :default 500.0))
  (bind _targetmilk (`self.targetMilk`))
  (`self.K2_DestroyActor`)
  (`/Engine/EditorBlueprintResources/StandardMacros.IsValid` _targetmilk
    (:`Is Valid`
      (set `/Game/Cats/BP_Milk.isTargeted` false _targetmilk))
    (:`Is Not Valid`
      _))
  (bind _outactors (`GameplayStatics.GetAllActorsOfClassWithTag` "/Script/Engine.TargetPoint" "CatRespawnArea"))
  (bind _randomlocation (`NavigationSystemV1.K2_GetRandomLocationInNavigableRadius` (`self.K2_GetActorLocation` (`KismetArrayLibrary.Array_Random` _outactors)) (`local.Radius`) null null))
  (`|SpawnActorFromClass` "BP_Cat1_C" (`KismetMathLibrary.Conv_VectorToTransform` _randomlocation) "AdjustIfPossibleButAlwaysSpawn" "MultiplyWithRoot" null null))

(fn `UserConstructionScript`)